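; Main player character for a shooter, with walk, sprint, strafe and backpedal speeds, jump, crouch, Alt free-look and a spring-arm aim zoom lerped on Tick (OnAim is false while aiming).
; On BeginPlay it spawns a BP_AR4 rifle on the hand socket, fired only when not sprinting.
; Damage feeds StatusAC, whose OnDeath plays a montage, drops the weapon, ragdolls and destroys the actor.
; Key 1 possesses BP_TestUnit actors.
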(event OnDeath(StatusAC)
  ;[1 1 1] Обработка смерти
  (Utilities|FlowControl|DoOnce false
    (:Completed
      (Collision|SetCollisionEnabled (Variables|Collision|GetCapsuleComponent) "NoCollision")
      (Animation|PlayAnimMontage "/Game/Main_Folder/Characters/Animation/Main/Death/DeathMontage.DeathMontage" 1.0 "None")
      (Transformation|DetachFromActor (Variables|Default|GetWeapon) "KeepRelative" "KeepRelative" "KeepRelative")
      (Utilities|FlowControl|Delay 2.3)
      (Physics|SetSimulatePhysics (Variables|Character|GetMesh) true)
      (Pawn|Components|CharacterMovement|DisableMovement (Variables|Character|GetCharacterMovement))
      (Utilities|FlowControl|Delay 4.0)
      (Actor|DestroyActor))))

(event Game|Damage|EventAnyDamage
  (params (Damage :type Float%20%28single-precision%29) (DamageType :type Damage%20Type%20Object%20Reference) (InstigatedBy :type Controller%20Object%20Reference) (DamageCauser :type Actor%20Object%20Reference))
  ;[1 1 1] Обработка нанесения урона
  (Default|MakeDamage/Health (Variables|Default|GetStatusAC) Damage))

(event EventBeginPlay
  ;[1 1 1] Прикрепления оружия со старта игры
  (CallFunction|SnapWeapon))

(event Game|Damage|EventPointDamage
  (params (Damage :type Float%20%28single-precision%29) (DamageType :type Damage%20Type%20Object%20Reference) (HitLocation :type Vector :default "0, 0, 0") (HitNormal :type Vector :default "0, 0, 0") (HitComponent :type Primitive%20Component%20Object%20Reference) (BoneName :type Name :default "None") (ShotFromDirection :type Vector :default "0, 0, 0") (InstigatedBy :type Controller%20Object%20Reference) (DamageCauser :type Actor%20Object%20Reference) (HitInfo :type Hit%20Result%20Structure%20%28by%20ref%29))
  (Variables|Default|SetLastPointDamageDirection ShotFromDirection)
  (Animation|Montage|PlayMontage (Variables|Character|GetMesh) "/Game/Main_Folder/Characters/Animation/Main/Move/Hit_Montage.Hit_Montage"))

(event EventTick
  (params (DeltaSeconds :type Float%20%28single-precision%29))
  (bind _springarm (Variables|Default|GetSpringArm))
  ;[0.4104 0.4301 1] Camera
  (if (Variables|Default|GetOnAim)
    (Variables|/Script/Engine.SpringArmComponent|SetTargetArmLength _springarm (Math|Float|Lerp (Variables|/Script/Engine.SpringArmComponent|GetTargetArmLength _springarm) 3.2e+02 0.2))
    (else
      (Variables|/Script/Engine.SpringArmComponent|SetTargetArmLength _springarm (Math|Float|Lerp (Variables|/Script/Engine.SpringArmComponent|GetTargetArmLength _springarm) 1.5e+02 0.1)))))

(event Input|ActionEvents|InputActionAim
  (params (Key :type Key%20Structure))
  ;[0.4104 0.4301 1] Camera
  ;;[1 1 1] Прицеливание
  (:Pressed
    (Variables|Default|SetOnAim false)
    (Variables|Default|SetisSprint? false))
  (:Released
    (Variables|Default|SetOnAim true)))

(event Input|ActionEvents|InputActionSprint
  (params (Key :type Key%20Structure))
  ;[1 0.7406 0.1876] Movemant
  ;;[1 1 1] Кнопка Спринта
  (:Pressed
    (if (== (stale Input|AxisEvents|InputAxisMoveForward AxisValue) 1.0)
      (Variables|Default|SetisSprint? true)
      (else
        (Variables|Default|SetisSprint? false))))
  (:Released
    (Variables|Default|SetisSprint? false)))

(event Input|ActionEvents|InputActionCrouch
  (params (Key :type Key%20Structure))
  ;[1 0.7406 0.1876] Movemant
  ;;[1 1 1] Возможность приседать
  (:Pressed
    (if (Variables|Default|GetbIsCrouched)
      (Character|UnCrouch)
      (else
        (Character|Crouch)))))

(event Input|ActionEvents|InputActionFire
  (params (Key :type Key%20Structure))
  (bind _weapon (Variables|Default|GetWeapon))
  ;[1 1 1] Кнопка Стрельбы
  (:Pressed
    (if (not (Variables|Default|GetisSprint?))
      (if true
        (Default|Firing _weapon true)
        (Animation|PlayAnimMontage "/Game/Main_Folder/Characters/Animation/Main/Move/Fire.Fire" 1.0 "None"))))
  (:Released
    (if (not (Variables|Default|GetisSprint?))
      (if true
        (Default|Firing _weapon false)
        (Animation|PlayAnimMontage "/Game/Main_Folder/Characters/Animation/Main/Move/Fire.Fire" 1.0 "None")))))

(event Input|ActionEvents|InputActionAim
  (params (Key :type Key%20Structure)))

(event Input|ActionEvents|InputActionJump
  (params (Key :type Key%20Structure))
  ;[1 0.7406 0.1876] Movemant
  ;;[1 1 1] Кнопка прыжка
  (:Pressed
    (if (Variables|Default|GetIsJump)
      (Character|StopJumping)
      (else
        (Character|Jump)))))

(event Input|AxisEvents|InputAxisMoveForward
  (params (AxisValue :type Float%20%28single-precision%29))
  ;[1 0.7406 0.1876] Movemant
  ;;[1 1 1] Передвижение
  (Pawn|Input|AddMovementInput (Math|Vector|GetForwardVector (Variables|Collision|GetCapsuleComponent)) AxisValue false)
  (Utilities|FlowControl|Sequence
    (:then_0
      ;;[1 1 1] Скорость ходьбы вперёд
      (Variables|/Script/Engine.CharacterMovementComponent|SetMaxWalkSpeed (Variables|Character|GetCharacterMovement) (Variables|Default|GetWalk%20Speed)))
    (:then_1
      ;;[1 1 1] Скорость ходьбы назад
      (if (== AxisValue -1.0)
        (Variables|/Script/Engine.CharacterMovementComponent|SetMaxWalkSpeed (Variables|Character|GetCharacterMovement) (Variables|Default|GetBackwardSpeed))))
    (:then_2
      ;;[1 1 1] Скорость бега
      (if (Variables|Default|GetisSprint?)
        (Variables|/Script/Engine.CharacterMovementComponent|SetMaxWalkSpeed (Variables|Character|GetCharacterMovement) (Variables|Default|GetSprintSpeed))))
    (:then_3
      ;;[1 1 1] Скорость стрейфа
      (if (Variables|Default|GetIsWalkRightleft)
        (Variables|/Script/Engine.CharacterMovementComponent|SetMaxWalkSpeed (Variables|Character|GetCharacterMovement) (Variables|Default|GetWalk%20Speed))))
    (:then_4
      ;;[1 1 1] Скорость бега назад
      (if (== AxisValue -1.0)
        (Variables|/Script/Engine.CharacterMovementComponent|SetMaxWalkSpeed (Variables|Character|GetCharacterMovement) (Variables|Default|GetBackwardSpeed))))))

(event Input|AxisEvents|InputAxisMoveRight
  (params (AxisValue :type Float%20%28single-precision%29))
  ;[1 0.7406 0.1876] Movemant
  ;;[1 1 1] Передвижение
  (Pawn|Input|AddMovementInput (Math|Vector|GetRightVector (Variables|Collision|GetCapsuleComponent)) AxisValue false)
  (Variables|Default|SetIsWalkRightleft (or (== AxisValue 1.0) (== AxisValue -1.0))))

(event Input|AxisEvents|InputAxisLookUp
  (params (AxisValue :type Float%20%28single-precision%29))
  ;[1 0.7406 0.1876] Movemant
  ;;[1 1 1] Управление мышью
  (Pawn|Input|AddControllerPitchInput AxisValue))

(event Input|AxisEvents|InputAxisLookRight
  (params (AxisValue :type Float%20%28single-precision%29))
  ;[1 0.7406 0.1876] Movemant
  ;;[1 1 1] Управление мышью
  (Pawn|Input|AddControllerYawInput AxisValue))

(event Input|KeyboardEvents|LeftAlt
  (params (Key :type Key%20Structure))
  ;[0.4104 0.4301 1] Camera
  ;;[1 1 1] Свободная камера
  (:Pressed
    (Variables|Default|SetbUseControllerRotationYaw false))
  (:Released
    (Variables|Default|SetbUseControllerRotationYaw true)))

(event Input|KeyboardEvents|1
  (params (Key :type Key%20Structure))
  (:Pressed
    (bind _outactors (Actor|GetAllActorsOfClass "/Game/Main_Folder/Characters/Game_characters/BP_TestUnit.BP_TestUnit_C"))
    (for _array_element _outactors
      (Pawn|Possess (Game|GetPlayerController 0) _array_element))))

(fn ConstructionScript)

(fn SnapWeapon
  (bind _returnvalue (Game|SpawnActorfromClass "/Game/Main_Folder/Damage/Weapon/BP_AR4.BP_AR4_C" (Transformation|GetWorldTransform (Variables|Character|GetMesh)) "Undefined" 0 0))
  (bind _output_get (Variables|Default|SetWeapon _returnvalue))
  (Transformation|AttachComponentToComponent _output_get (Variables|Character|GetMesh) "Socket_gun" "SnapToTarget" "SnapToTarget" "SnapToTarget" true))