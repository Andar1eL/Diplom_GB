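; M4 weapon Blueprint whose Firing event, when toggled on, spends ammo through AmmoAC to play shot sound and muzzle flash, or an empty-magazine sound.
; Each attempt refreshes the ammo text and is gated by a FireDelay flag.
; The fire-rate delay that clears this flag and loops back is unconnected, so nothing here resets it.
; SpawnProjectile spawns BP_Ammo at the Arrow but is not called in this file.
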(event Custom|Firing
  (params (Toggle :type Boolean))
  (bind _ammoac (Variables|Default|GetAmmoAC))
  (bind _ammoac_2 (Variables|Default|GetAmmoAC))
  (bind _output_get (Variables|Default|SetCanFire Toggle))
  (if _output_get
    (if (and (Variables|Default|GetCanFire) (not (Variables|Default|GetFireDelay)))
      (Variables|Default|SetFireDelay true)
      (Utilities|FlowControl|Sequence
        (:then_0
          (if (Default|CheckAmmo _ammoac 1)
            (Default|SubstractAmmo _ammoac 1)
            ;[1 1 1] Воспроизведение звука при выстреле
            (Audio|SpawnSoundatLocation "/Game/Main_Folder/Damage/Weapon/Sounds/Shot_AR4.Shot_AR4" (Transformation|GetWorldLocation (Variables|Default|GetWeapon)) "0, 0, 0" 1.0 1.0 0.0 0 0)
            ;[1 1 1] Создание эффект частиц из дула
            (Effects|SpawnEmitteratLocation "/Game/Realistic_Starter_VFX_Pack_Vol2/Particles/Hit/P_Default.P_Default" (Transformation|GetSocketLocation (Variables|Default|GetWeapon) "b_gun_muzzleflash") (Transformation|GetSocketRotation (Variables|Default|GetWeapon) "b_gun_muzzleflash") "0.500000,1.000000,1.000000")
            (else
              ;[1 1 1] Звук при пустом магазине
              (Audio|SpawnSoundatLocation "/Game/Main_Folder/Audio/EmptyAmmo.EmptyAmmo" (Transformation|GetActorLocation) "0, 0, 0" 1.0 1.0 0.0 0 0))))
        (:then_1
          (Rendering|Components|TextRender|SetText (Variables|Default|GetAmmoText) (Utilities|Text|FormatText "{Current}/{Max}" (Variables|/Game/Main_Folder/Damage/Weapon/AmmoAC.AmmoAC_C|GetCurrentAmmo _ammoac_2) (Variables|/Game/Main_Folder/Damage/Weapon/AmmoAC.AmmoAC_C|GetMaxAmmo _ammoac_2))))))))

(fn ConstructionScript
  (|CallParentFunction))

(fn SpawnProjectile
  (Game|SpawnActorfromClass "/Game/Main_Folder/Damage/Weapon/BP_Ammo.BP_Ammo_C" (Transformation|GetWorldTransform (Variables|Default|GetArrow)) "AlwaysSpawn" 0 0))