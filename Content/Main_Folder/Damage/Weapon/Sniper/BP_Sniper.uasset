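; BP_Sniper is a sniper rifle weapon that fires automatically at a fixed slow rate while its fire toggle is on.
; The Fire event stores the toggle and loops through a delay, with a FireDelay flag blocking overlapping shots.
; Each shot spawns a BP_SniperBullet at the skeletal mesh's Muzzle socket, plays the shot sound and emits a muzzle effect at the suppressor component.
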(event Custom|Fire
  (params (Toggle :type Boolean))
  (bind _suppressoor (Variables|Default|GetSuppressoor))
  (bind _output_get (Variables|Default|SetCanFire Toggle))
  (if _output_get
    (if (and (Variables|Default|GetCanFire) (not (Variables|Default|GetFireDelay))) :!label _label
      (Variables|Default|SetFireDelay true)
      (CallFunction|SpawnProhectile)
      ;[1 1 1] Звук выстрела
      (Audio|SpawnSoundatLocation "/Game/Main_Folder/Damage/Weapon/Sniper/S_SniperShot.S_SniperShot" (Transformation|GetActorLocation) "0, 0, 0" 1.0 1.0 0.0 0 0)
      ;[1 1 1] Эффект выстрела
      (Effects|SpawnEmitteratLocation "/Game/Main_Folder/Damage/Weapon/PS_Muzzle.PS_Muzzle" (Transformation|GetWorldLocation _suppressoor) (Transformation|GetWorldRotation _suppressoor))
      (Utilities|FlowControl|Delay 3.0)
      (Variables|Default|SetFireDelay false)
      (goto _label))))

(event EventBeginPlay)

(event Collision|EventActorBeginOverlap
  (params (OtherActor :type Actor%20Object%20Reference)))

(event EventTick
  (params (DeltaSeconds :type Float%20%28single-precision%29)))

(fn ConstructionScript)

(fn SpawnProhectile
  (Game|SpawnActorfromClass "/Game/Main_Folder/Damage/Weapon/BP_SniperBullet.BP_SniperBullet_C" (Transformation|GetSocketTransform (Variables|Default|GetSkeletalMesh) "Muzzle" "RTS_World") "Undefined" 0 0))