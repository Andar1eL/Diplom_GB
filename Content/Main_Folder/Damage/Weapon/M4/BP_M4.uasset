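; BP_M4 is an automatic M4 rifle weapon actor that fires while its Fire event toggle is on.
; A self-looping Delay with a FireDelay guard sets the fire rate, repeating until CanFire turns off.
; Each shot spawns a BP_Ammo projectile at the "Dulo" socket, plays a shot sound at the actor and spawns a muzzle flash emitter at the muzzle socket.
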(event Custom|Fire
  (params (Toggle :type Boolean))
  (bind _skeletalmesh (Variables|Default|GetSkeletalMesh))
  (bind _output_get (Variables|Default|SetCanFire Toggle))
  (if _output_get
    (if (and (Variables|Default|GetCanFire) (not (Variables|Default|GetFireDelay))) :!label _label
      (Variables|Default|SetFireDelay true)
      (CallFunction|SpawnProjectile)
      ;[1 1 1] Звук выстрела
      (Audio|SpawnSoundatLocation "/Game/Main_Folder/Damage/Weapon/M4/Shot_AR4.Shot_AR4" (Transformation|GetActorLocation) "0, 0, 0" 1.0 1.0 0.0 0 0)
      ;[1 1 1] Эффект выстрела
      (Effects|SpawnEmitteratLocation "/Game/Main_Folder/Damage/Weapon/PS_Muzzle.PS_Muzzle" (Transformation|GetSocketLocation _skeletalmesh "b_gun_muzzleflash") (Transformation|GetSocketRotation _skeletalmesh "b_gun_muzzleflash"))
      (Utilities|FlowControl|Delay 0.2)
      (Variables|Default|SetFireDelay false)
      (goto _label))))

(event EventBeginPlay)

(event Collision|EventActorBeginOverlap
  (params (OtherActor :type Actor%20Object%20Reference)))

(event EventTick
  (params (DeltaSeconds :type Float%20%28single-precision%29)))

(fn ConstructionScript)

(fn SpawnProjectile
  (Game|SpawnActorfromClass "/Game/Main_Folder/Damage/Weapon/BP_Ammo.BP_Ammo_C" (Transformation|GetSocketTransform (Variables|Default|GetSkeletalMesh) "Dulo" "RTS_World") "Undefined" 0 0))